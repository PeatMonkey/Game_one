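; NPC AI controller that starts patrol behavior and reports what the pawn perceives.
; On BeginPlay it applies the Patrol_Data blackboard and runs the Patrol behavior tree.
; AI Perception updates print the pawn, sense class and sensed actor for debugging.
; FindPatrolRoute looks unfinished: it casts the pawn to ThirdPersonCharacter, then sets the Waypoint key without a value, leaving PatrolRoutes unused.
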(event `self.ReceiveBeginPlay`
  ;[1 1 1] AI Patrolling
  (`self.UseBlackboard` "/Game/Patrol_Data.Patrol_Data")
  (`self.RunBehaviorTree` "/Game/Patrol.Patrol"))

(event `self.AIPerception.OnTargetPerceptionUpdated`
  (params (Actor :type "Actor Object Reference") (Stimulus :type "AIStimulus Structure"))
  ;[1 1 1] Print what the AI Sees
  (bind _returnvalue (`AIPerceptionSystem.GetSenseClassForStimulus` Stimulus))
  (`KismetSystemLibrary.PrintString` (`KismetStringLibrary.Concat_StrStr` (`KismetSystemLibrary.GetObjectName` (`self.K2_GetPawn`)) " " (`KismetSystemLibrary.GetClassDisplayName` _returnvalue) " " (`KismetSystemLibrary.GetObjectName` Actor))))

(fn `FindPatrolRoute`
  (params (self2 :type "BlackboardComponent Object Reference"))
  (bind _asthird_person_character (cast `/Game/ThirdPersonCPP/Blueprints/ThirdPersonCharacter` (`self.K2_GetPawn`)))
  (`BlackboardComponent.SetValueAsObject` self2 "Waypoint" null))

(fn `UserConstructionScript`)