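; Behavior tree task that picks the next patrol waypoint for an AI-controlled ThirdPersonCharacter.
; It reads the pawn's PatrolRoutes, uses the blackboard Index to select a point and writes it to the Waypoint key.
; It then advances Index with a modulo on the route length, so the patrol loops, and finishes with success.
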(event `self.ReceiveExecuteAI`
  (params (OwnerController :type "AIController Object Reference") (ControlledPawn :type "Pawn Object Reference"))
  (`self.GetPstrolPoints` ControlledPawn)
  ;[1 1 1] Set Next Waypoint
  (bind _index (`self.NextWaypoint`))
  ;[1 1 1] Cycle Index
  (`self.CycleIndex` _index)
  (`self.FinishExecute` true))

(fn `CycleIndex`
  (params (A :type Integer))
  (`BTFunctionLibrary.SetBlackboardValueAsInt` (`self.Index`) (mod (+ A 1) (`KismetArrayLibrary.Array_Length` (`self.Patrol Points`)))))

(fn `GetPstrolPoints`
  (params (Object :type "Object Object Reference"))
  (bind _asthird_person_character (cast `/Game/ThirdPersonCPP/Blueprints/ThirdPersonCharacter` Object))
  (set `self.Patrol Points` (`/Game/ThirdPersonCPP/Blueprints/ThirdPersonCharacter.Patrol Routes` _asthird_person_character)))

(fn `NextWaypoint`
  (returns (index :type Integer))
  (bind _returnvalue (`BTFunctionLibrary.GetBlackboardValueAsInt` (`self.Index`)))
  (`BTFunctionLibrary.SetBlackboardValueAsObject` (`self.Waypoint`) (`KismetArrayLibrary.Array_Get` (`self.Patrol Points`) _returnvalue))
  (return _returnvalue))